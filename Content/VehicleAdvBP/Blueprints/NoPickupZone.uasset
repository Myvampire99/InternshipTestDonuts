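; NoPickupZone is a trigger volume that blocks a vehicle from picking up the ball while inside it.
; On actor overlap begin and end it casts the other actor to VehicleBlueprint and toggles its CanPickupBall flag off and back on.
; The toggle only applies when that vehicle is the pawn of the player matching the zone's PlayerID, so each zone restricts one specific player.
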(event Collision|EventActorBeginOverlap
  (params (OtherActor :type Actor%20Object%20Reference))
  ;[1 1 1] BeginOverlap
  (bind _asvehicle_blueprint (Utilities|Casting|CastToVehicleBlueprint OtherActor))
  (if (== _asvehicle_blueprint (Game|Player|GetPlayerPawn (Variables|Default|GetPlayerID)))
    (Variables|/Game/VehicleAdvBP/Blueprints/VehicleBlueprint.VehicleBlueprint_C|SetCanPickupBall _asvehicle_blueprint false)))

(event Collision|EventActorEndOverlap
  (params (OtherActor :type Actor%20Object%20Reference))
  ;[1 1 1] EndOverlap
  (bind _asvehicle_blueprint (Utilities|Casting|CastToVehicleBlueprint OtherActor))
  (if (== _asvehicle_blueprint (Game|Player|GetPlayerPawn (Variables|Default|GetPlayerID)))
    (Variables|/Game/VehicleAdvBP/Blueprints/VehicleBlueprint.VehicleBlueprint_C|SetCanPickupBall _asvehicle_blueprint true)))

(fn ConstructionScript)